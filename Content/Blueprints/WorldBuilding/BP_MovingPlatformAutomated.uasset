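; Automated moving platform that shuttles its Cube back and forth in an endless loop from BeginPlay.
; A timeline lerps between StartTransform and EndTransform, driving relative location, offset by the actor's starting world position, and relative rotation.
; A FlipFlop on the timeline's Finished output alternates reverse and forward playback.
; An Activate event resets the Cube to its start transform, sets Ended and sets the timeline's time.
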(event Custom|BackToStart
  ;[1 1 1] Moving Animation
  (bind _alpha_value (Timeline|Move_TimeLine Reverse)
    (:Update
      (Transformation|SetRelativeLocation (Variables|Default|GetCube) (+ (Variables|Default|GetStartWorldPos) (.location (Math|Transform|Lerp(Transform) (Variables|Default|GetStartTransform) (Variables|Default|GetEndTransform) _alpha_value))) false false)
      (Transformation|SetRelativeRotation (Variables|Default|GetCube) (.rotation (Math|Transform|Lerp(Transform) (Variables|Default|GetStartTransform) (Variables|Default|GetEndTransform) _alpha_value)) false false))
    (:Finished
      ;[1 1 1] Infinite moving loop
      (Utilities|FlowControl|FlipFlop
        (:A
          (CallFunction|BacktoStart))
        (:B
          (CallFunction|MovetoPoint))))))

(event Custom|MoveToPoint
  ;[1 1 1] Moving Animation
  (bind _alpha_value (Timeline|Move_TimeLine Play)
    (:Update
      (Transformation|SetRelativeLocation (Variables|Default|GetCube) (+ (Variables|Default|GetStartWorldPos) (.location (Math|Transform|Lerp(Transform) (Variables|Default|GetStartTransform) (Variables|Default|GetEndTransform) _alpha_value))) false false)
      (Transformation|SetRelativeRotation (Variables|Default|GetCube) (.rotation (Math|Transform|Lerp(Transform) (Variables|Default|GetStartTransform) (Variables|Default|GetEndTransform) _alpha_value)) false false))
    (:Finished
      ;[1 1 1] Infinite moving loop
      (Utilities|FlowControl|FlipFlop
        (:A
          (CallFunction|BacktoStart))
        (:B
          (CallFunction|MovetoPoint))))))

(event EventActivate
  (params (ActualArenaIndex :type Integer))
  (bind _starttransform (Variables|Default|GetStartTransform))
  ;[1 1 1] Reset Platform
  (Transformation|SetRelativeTransform (Variables|Default|GetCube) (Math|Transform|MakeTransform (+ (Variables|Default|GetStartWorldPos) (.location _starttransform)) (.rotation _starttransform) (.scale _starttransform)) false false)
  (Variables|Default|SetEnded? true)
  ;[1 1 1] Moving Animation
  (bind _alpha_value (Timeline|Move_TimeLine SetNewTime)
    (:Update
      (Transformation|SetRelativeLocation (Variables|Default|GetCube) (+ (Variables|Default|GetStartWorldPos) (.location (Math|Transform|Lerp(Transform) (Variables|Default|GetStartTransform) (Variables|Default|GetEndTransform) _alpha_value))) false false)
      (Transformation|SetRelativeRotation (Variables|Default|GetCube) (.rotation (Math|Transform|Lerp(Transform) (Variables|Default|GetStartTransform) (Variables|Default|GetEndTransform) _alpha_value)) false false))
    (:Finished
      ;[1 1 1] Infinite moving loop
      (Utilities|FlowControl|FlipFlop
        (:A
          (CallFunction|BacktoStart))
        (:B
          (CallFunction|MovetoPoint))))))

(event EventBeginPlay
  ;[1 1 1] BEGIN PLAY: Set World Location Variable
  (Variables|Default|SetStartWorldPos (Transformation|GetActorLocation))
  (CallFunction|MovetoPoint))

(fn ConstructionScript)