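; Moving platform Blueprint that travels between a start and end transform each time a Player-tagged actor enters its trigger.
; An Ended flag ignores touches mid-move, while a flip-flop boolean alternates playing and reversing one timeline.
; The timeline lerps the Cube's location and rotation, offsetting its relative location by the actor position cached at BeginPlay.
; Activate resets the Cube, flags and timeline to the start state.
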(event OnComponentBeginOverlap(MoveTrigger)
  (params (OverlappedComponent :type Primitive%20Component%20Object%20Reference) (OtherActor :type Actor%20Object%20Reference) (OtherComp :type Primitive%20Component%20Object%20Reference) (OtherBodyIndex :type Integer) (bFromSweep :type Boolean) (SweepResult :type Hit%20Result%20Structure%20%28by%20ref%29))
  ;[1 1 1] Move platform on player overlap
  (if (Actor|ActorHasTag OtherActor "Player")
    (if (Variables|Default|GetEnded?)
      (Variables|Default|SetEnded? false)
      (bind _output_get (Variables|Default|SetFlipFlopCustom (not (Variables|Default|GetFlipFlopCustom))))
      (if _output_get
        (CallFunction|MovetoPoint)
        (else
          (CallFunction|BacktoStart))))))

(event Custom|BackToStart
  ;[1 1 1] Moving Animation
  (bind _alpha_value (Timeline|Move_TimeLine Reverse)
    (:Update
      (Transformation|SetRelativeLocation (Variables|Default|GetCube) (+ (Variables|Default|GetStartWorldPos) (.location (Math|Transform|Lerp(Transform) (Variables|Default|GetStartTransform) (Variables|Default|GetEndTransform) _alpha_value))) false false)
      (Transformation|SetRelativeRotation (Variables|Default|GetCube) (.rotation (Math|Transform|Lerp(Transform) (Variables|Default|GetStartTransform) (Variables|Default|GetEndTransform) _alpha_value)) false false))
    (:Finished
      (Variables|Default|SetEnded? true))))

(event Custom|MoveToPoint
  ;[1 1 1] Moving Animation
  (bind _alpha_value (Timeline|Move_TimeLine Play)
    (:Update
      (Transformation|SetRelativeLocation (Variables|Default|GetCube) (+ (Variables|Default|GetStartWorldPos) (.location (Math|Transform|Lerp(Transform) (Variables|Default|GetStartTransform) (Variables|Default|GetEndTransform) _alpha_value))) false false)
      (Transformation|SetRelativeRotation (Variables|Default|GetCube) (.rotation (Math|Transform|Lerp(Transform) (Variables|Default|GetStartTransform) (Variables|Default|GetEndTransform) _alpha_value)) false false))
    (:Finished
      (Variables|Default|SetEnded? true))))

(event EventActivate
  (params (ActualArenaIndex :type Integer))
  (bind _starttransform (Variables|Default|GetStartTransform))
  ;[1 1 1] Reset Platform
  (Variables|Default|SetFlipFlopCustom false)
  (Transformation|SetRelativeTransform (Variables|Default|GetCube) (Math|Transform|MakeTransform (+ (Variables|Default|GetStartWorldPos) (.location _starttransform)) (.rotation _starttransform) (.scale _starttransform)) false false)
  (Variables|Default|SetEnded? true)
  (Utilities|FlowControl|Sequence
    (:then_0
      ;[1 1 1] Moving Animation
      (bind _alpha_value (Timeline|Move_TimeLine Stop)
        (:Update
          (Transformation|SetRelativeLocation (Variables|Default|GetCube) (+ (Variables|Default|GetStartWorldPos) (.location (Math|Transform|Lerp(Transform) (Variables|Default|GetStartTransform) (Variables|Default|GetEndTransform) _alpha_value))) false false)
          (Transformation|SetRelativeRotation (Variables|Default|GetCube) (.rotation (Math|Transform|Lerp(Transform) (Variables|Default|GetStartTransform) (Variables|Default|GetEndTransform) _alpha_value)) false false))
        (:Finished
          (Variables|Default|SetEnded? true))))
    (:then_1
      (Timeline|Move_TimeLine SetNewTime))))

(event EventBeginPlay
  ;[1 1 1] BEGIN PLAY = Set World Location Variable
  (Variables|Default|SetStartWorldPos (Transformation|GetActorLocation)))

(fn ConstructionScript)