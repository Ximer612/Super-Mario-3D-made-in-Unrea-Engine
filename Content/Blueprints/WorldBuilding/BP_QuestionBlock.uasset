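; BP_QuestionBlock is a question block that the player hits from below to possibly release a random pickup.
; A Player-tagged hit with an upward impact normal hides the cube, disables its collision, swaps its material and randomly spawns an item from PickupItemsActors, or nothing.
; Activate restores the block and destroys its spawned pickup when the given arena index is at or below the block's own.
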(event OnComponentHit(Cube)
  (params (HitComponent :type Primitive%20Component%20Object%20Reference) (OtherActor :type Actor%20Object%20Reference) (OtherComp :type Primitive%20Component%20Object%20Reference) (NormalImpulse :type Vector :default "0, 0, 0") (Hit :type Hit%20Result%20Structure%20%28by%20ref%29))
  ;[1 1 1] When Player hits this block from below
  (if (Actor|ActorHasTag OtherActor "Player")
    (if (Math|Vector|Equal(Vector) (.impactnormal Hit) "0.000000, 0,1.000000" 0.0001)
      (CallFunction|Deactivate)
      (CallFunction|SpawnRandomPickuporNone (Transformation|GetWorldTransform (Variables|Default|GetCube))))))

(event Custom|SpawnRandomPickupOrNone
  (params (NewPickupTransform :type Transform))
  (bind _pickupitemsactors (Variables|Default|GetPickupItemsActors))
  ;[1 1 1] Summon random pickup
  (if (> (Math|Random|RandomInteger 100) 30)
    (bind _returnvalue (Game|SpawnActorfromClass (Utilities|Array|Get(acopy) _pickupitemsactors (Math|Random|RandomInteger (Utilities|Array|Length _pickupitemsactors))) NewPickupTransform "AlwaysSpawn" 0 0))
    (Variables|Default|SetSpawnedPickupItem _returnvalue)))

(event EventActivate
  (params (ActualArenaIndex :type Integer))
  (bind _cube (Variables|Default|GetCube))
  ;[1 1 1] Enable / Disable mesh
  (if (<= ActualArenaIndex (Variables|Default|GetMyArenaIndex))
    (Collision|SetCollisionEnabled _cube "QueryAndPhysics")
    (Development|SetHiddeninGame _cube false false)
    (Rendering|Material|SetMaterial (Variables|Default|GetCube) 0 (Variables|Default|GetDefaultMaterial))
    ;;[1 1 1] If has released a pickup and it's active destroy it
    (Utilities|IsValid (Variables|Default|GetSpawnedPickupItem)
      (:Is%20Valid
        (Actor|DestroyActor (Variables|Default|GetSpawnedPickupItem))))))

(event EventDeactivate
  (bind _cube (Variables|Default|GetCube))
  ;[1 1 1] Enable / Disable mesh
  (Collision|SetCollisionEnabled _cube "NoCollision")
  (Development|SetHiddeninGame _cube true false)
  (Rendering|Material|SetMaterial (Variables|Default|GetCube) 0 (Variables|Default|GetInteractedMaterial)))

(fn ConstructionScript)