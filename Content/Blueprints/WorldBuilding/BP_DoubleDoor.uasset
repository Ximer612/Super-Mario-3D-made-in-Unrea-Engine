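; BP_DoubleDoor is a two-leaf swinging door tied to an arena index.
; Open plays a timeline that lerps both leaves by shortest path from their start rotations to a shared end rotation, and Close reverses it.
; Activate resets the door when the given arena index is at or below its own, restoring closed rotations, clearing ShouldBeOpen and stopping the timeline.
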(event Custom|Close
  ;[1 1 1] Open Doors Animation
  (bind _alpha (Timeline|Doors_Timeline Reverse)
    (:Update
      (Transformation|SetRelativeRotation (Variables|Default|GetDoorRight) (Math|Rotator|Lerp(Rotator) (Variables|Default|GetStartRotation) (Variables|Default|GetEndRotation) _alpha true) false false)
      (Transformation|SetRelativeRotation (Variables|Default|GetDoorLeft) (Math|Rotator|Lerp(Rotator) (Variables|Default|GetStartLeftDoor) (Variables|Default|GetEndRotation) _alpha true) false false))))

(event Custom|Open
  ;[1 1 1] Open Doors Animation
  (bind _alpha (Timeline|Doors_Timeline PlayFromStart)
    (:Update
      (Transformation|SetRelativeRotation (Variables|Default|GetDoorRight) (Math|Rotator|Lerp(Rotator) (Variables|Default|GetStartRotation) (Variables|Default|GetEndRotation) _alpha true) false false)
      (Transformation|SetRelativeRotation (Variables|Default|GetDoorLeft) (Math|Rotator|Lerp(Rotator) (Variables|Default|GetStartLeftDoor) (Variables|Default|GetEndRotation) _alpha true) false false))))

(event Custom|ResetDoors
  ;[1 1 1] Reset Doors
  (Transformation|SetRelativeRotation (Variables|Default|GetDoorRight) "0, 0, 0" false false)
  (Transformation|SetRelativeRotation (Variables|Default|GetDoorLeft) (Variables|Default|GetStartLeftDoor) false false)
  (Variables|Default|SetShouldBeOpen? false)
  (CallFunction|StopAnimation))

(event Custom|StopAnimation
  ;[1 1 1] Open Doors Animation
  (bind _alpha (Timeline|Doors_Timeline Stop)
    (:Update
      (Transformation|SetRelativeRotation (Variables|Default|GetDoorRight) (Math|Rotator|Lerp(Rotator) (Variables|Default|GetStartRotation) (Variables|Default|GetEndRotation) _alpha true) false false)
      (Transformation|SetRelativeRotation (Variables|Default|GetDoorLeft) (Math|Rotator|Lerp(Rotator) (Variables|Default|GetStartLeftDoor) (Variables|Default|GetEndRotation) _alpha true) false false))))

(event EventActivate
  (params (ActualArenaIndex :type Integer))
  ;[1 1 1] Reset Doors
  (if (<= ActualArenaIndex (Variables|Default|GetMyArenaIndex))
    (CallFunction|ResetDoors)))

(fn ConstructionScript)