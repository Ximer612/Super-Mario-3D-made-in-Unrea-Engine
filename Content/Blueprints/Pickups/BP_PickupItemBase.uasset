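; Base Blueprint for pickup items, with a physics-capable box for overlap detection and a billboard as its visual.
; Any overlap on the box fires OnPickup, which calls Deactivate to turn off physics and collision and hide the billboard.
; Activate restores all three only when the passed arena index is less than or equal to the item's own arena index.
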(event OnComponentBeginOverlap(Box)
  (params (OverlappedComponent :type Primitive%20Component%20Object%20Reference) (OtherActor :type Actor%20Object%20Reference) (OtherComp :type Primitive%20Component%20Object%20Reference) (OtherBodyIndex :type Integer) (bFromSweep :type Boolean) (SweepResult :type Hit%20Result%20Structure%20%28by%20ref%29))
  ;[1 1 1] Check collision and on pickup
  (CallFunction|OnPickup))

(event Custom|OnPickup
  ;[1 1 1] Check collision and on pickup
  (CallFunction|Deactivate))

(event EventActivate
  (params (ActualArenaIndex :type Integer))
  (bind _box (Variables|Default|GetBox))
  ;[1 1 1] Enable/Disable this
  (if (<= ActualArenaIndex (Variables|Custom|GetMyArenaIndex))
    (Physics|SetSimulatePhysics _box true)
    (Collision|SetCollisionEnabled _box "QueryAndPhysics")
    (Development|SetHiddeninGame (Variables|Default|GetBillboard) false false)))

(event EventDeactivate
  (bind _box (Variables|Default|GetBox))
  ;[1 1 1] Enable/Disable this
  (Physics|SetSimulatePhysics _box false)
  (Collision|SetCollisionEnabled _box "NoCollision")
  (Development|SetHiddeninGame (Variables|Default|GetBillboard) true false))

(fn ConstructionScript)