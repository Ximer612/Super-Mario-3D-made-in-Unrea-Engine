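; Boss enemy Blueprint that stays deactivated until the area-unlocked dispatcher reports its own arena index.
; It is immortal, via a capsule collision object type swap, until accumulated target steps reach their maximum.
; A hit while vulnerable applies damage, picks walk speed from remaining health, clears the blackboard tired flag, restores immortality and plays the spin animation.
; Resetting the step count plays a looping pain animation.
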(event Custom|SetImmortal
  (params (IsImmortal? :type Boolean))
  ;[1 1 1] Can player hit the boss?
  (bind _output_get (Variables|Default|SetIs%20Immortal? IsImmortal?))
  (if _output_get
    (Collision|SetCollisionObjectType (Variables|Default|GetCapsuleComponent) "ECC_WorldDynamic")
    (else
      (Collision|SetCollisionObjectType (Variables|Default|GetCapsuleComponent) "ECC_GameTraceChannel3"))))

(event Custom|SpawnBoss
  ;[1 1 1] Spawns Boss when all areas are completed
  (CallFunction|Activate (Variables|/Game/Blueprints/BP_ArenasController.BP_ArenasController_C|GetActualArenaIndex (Variables|Default|GetEventDispatcherSenderRef))))

(event Custom|SetWalkSpeed
  (params (Index :type Integer))
  ;[1 1 1] Change movement speed
  (Variables|/Script/Engine.CharacterMovementComponent|SetMaxWalkSpeed (Variables|Character|GetCharacterMovement) (Utilities|Array|Get(acopy) (Variables|Default|GetWalkSpeeds) Index)))

(event EventBeginPlay
  ;[1 1 1] BEGIN PLAY = set walk speed and immortal to true
  (|CallParentFunction)
  (CallFunction|SetWalkSpeed (Variables|Default|GetMyArenaIndex))
  ;[1 1 1] Spawns Boss when all areas are completed
  (CallFunction|SetImmortal true)
  (EventDispatchers|BindEventtoNewAreaUnlocked (Variables|Default|GetEventDispatcherSenderRef) (delegate Custom|SpawnBoss))
  (CallFunction|Deactivate))

(event EventActivate
  (params (ActualArenaIndex :type Integer))
  (bind _myarenaindex (Variables|Default|GetMyArenaIndex))
  ;[1 1 1] activate only in the boss area index not before
  (if (== ActualArenaIndex _myarenaindex)
    (|CallParentFunction _myarenaindex)
    (else
      (CallFunction|Deactivate))))

(event EventResetTargetSteps
  ;[1 1 1] Restart the target count when reached the max
  (Variables|Default|SetTargetSteps 0)
  (Components|Animation|PlayAnimation (Variables|Character|GetMesh) "/Game/Models/Bowser/Anim_Pain.Anim_Pain" true))

(event Game|Damage|EventAnyDamage
  (params (Damage :type Float%20%28single-precision%29) (DamageType :type Damage%20Type%20Object%20Reference) (InstigatedBy :type Controller%20Object%20Reference) (DamageCauser :type Actor%20Object%20Reference))
  ;[1 1 1] Check boss damage taken and IA
  (if (not (Variables|Default|GetIs%20Immortal?))
    (|CallParentFunction Damage DamageType InstigatedBy DamageCauser)
    (CallFunction|SetWalkSpeed (Math|Float|Truncate (Variables|Default|GetHealth)))
    (AI|Components|Blackboard|SetValueasBool (AI|GetBlackboard (Pawn|GetController)) (Variables|Default|GetIsTired) false)
    (CallFunction|SetImmortal true)
    (CallFunction|Spin)))

(event EventSpin
  ;[1 1 1] Spin boss with interface to not cast
  (Components|Animation|PlayAnimation (Variables|Character|GetMesh) "/Game/Models/Bowser/Anim_Spin.Anim_Spin" true))

(fn ConstructionScript
  (|CallParentFunction))

(fn AddandCheckSteps
  (params (StepNum :type Integer))
  (bind _output_get (Variables|Default|SetTargetSteps (+ (Variables|Default|GetTargetSteps) StepNum)))
  (if (>= _output_get (Variables|Default|GetMaxTargetSteps))
    (CallFunction|SetImmortal false))
  (return (>= _output_get (Variables|Default|GetMaxTargetSteps))))