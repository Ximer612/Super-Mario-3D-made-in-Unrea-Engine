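; AI controller for the Advanced Walker enemy that runs its behavior tree on possess and tracks sight of the player.
; Perception updates for actors tagged Player set the line-of-sight flag and player reference on the Blackboard.
; Losing the player starts a timer that clears both keys after a grace period, and sensing the player again cancels it.
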(event OnTargetPerceptionUpdated(AIPerception)
  (params (Actor :type Actor%20Object%20Reference) (Stimulus :type AI%20Stimulus%20Structure))
  (bind _blackboard (Variables|Default|GetBlackboard))
  ;[1 1 1] CHECK IF THA AI PERCEPTION HAVE SEEN PLAYER AND HAS SUCCESFULLY SENSED
  (if (Actor|ActorHasTag Actor "Player")
    (if (Utilities|Struct|BreakAIStimulus Stimulus)
      ;[1 1 1] TRUE
      (Utilities|Time|ClearandInvalidateTimerbyHandle (Variables|Default|GetResetSightTimer))
      (AI|Components|Blackboard|SetValueasBool _blackboard (Variables|Default|GetHasLineOfSight) true)
      (AI|Components|Blackboard|SetValueasObject _blackboard (Variables|Default|GetPlayerRef) Actor)
      (else
        ;[1 1 1] FALSE
        (bind _returnvalue (Utilities|Time|SetTimerbyEvent (delegate Custom|ResetLineOfSight) (Variables|Default|GetResetSightTime)))
        (Variables|Default|SetResetSightTimer _returnvalue)))))

(event Custom|ResetLineOfSight
  (bind _blackboard (Variables|Default|GetBlackboard))
  ;[1 1 1] FALSE
  (AI|Components|Blackboard|SetValueasBool _blackboard (Variables|Default|GetHasLineOfSight) false)
  (AI|Components|Blackboard|SetValueasObject _blackboard (Variables|Default|GetPlayerRef) 0))

(event EventPossess
  (params (PossessedPawn :type Pawn%20Object%20Reference))
  (Variables|Default|SetPossessed%20Pawn PossessedPawn)
  (AI|RunBehaviorTree "/Game/Blueprints/Enemy/AdvancedWalker/BT_AdvancedWalkerEnemy.BT_AdvancedWalkerEnemy"))

(fn ConstructionScript)