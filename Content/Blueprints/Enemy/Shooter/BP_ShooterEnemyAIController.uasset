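; AI controller for the shooter enemy that runs BT_ShooterEnemy on possess and drives its sight and shooting blackboard keys.
; When perception senses the player, it stores the player reference and line of sight, then starts a looping timer that sets ShouldShoot by distance to the player.
; On losing the player, it stops shooting immediately but clears line of sight and the reference only after a delay.
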(event OnTargetPerceptionUpdated(AIPerception)
  (params (Actor :type Actor%20Object%20Reference) (Stimulus :type AI%20Stimulus%20Structure))
  (bind _blackboard (Variables|Default|GetBlackboard))
  (if (Actor|ActorHasTag Actor "Player")
    (if (Utilities|Struct|BreakAIStimulus Stimulus)
      ;[1 1 1] TRUE = Enemy can see player
      (Utilities|Time|ClearandInvalidateTimerbyHandle (Variables|Default|GetResetSightTimer))
      (AI|Components|Blackboard|SetValueasBool _blackboard (Variables|Default|GetHasLineOfSight) true)
      (AI|Components|Blackboard|SetValueasObject _blackboard (Variables|Default|GetPlayerRef) Actor)
      (bind _returnvalue (Utilities|Time|SetTimerbyEvent (delegate Custom|RangedAttack) (Variables|Default|GetRangedAttackTime) true))
      (Variables|Default|SetRangedAttackTimer _returnvalue)
      (else
        ;[1 1 1] FALSE = Enemy cant see Player
        (bind _returnvalue_2 (Utilities|Time|SetTimerbyEvent (delegate Custom|ResetLineOfSight) (Variables|Default|GetResetSightTime)))
        (Variables|Default|SetResetSightTimer _returnvalue_2)
        (AI|Components|Blackboard|SetValueasBool (Variables|Default|GetBlackboard) (Variables|Default|GetShouldShoot) false)
        (Utilities|Time|ClearandInvalidateTimerbyHandle (Variables|Default|GetRangedAttackTimer))))))

(event Custom|ResetLineOfSight
  (bind _blackboard (Variables|Default|GetBlackboard))
  ;[1 1 1] FALSE = Enemy cant see Player
  (AI|Components|Blackboard|SetValueasBool _blackboard (Variables|Default|GetHasLineOfSight) false)
  (AI|Components|Blackboard|SetValueasObject _blackboard (Variables|Default|GetPlayerRef) 0))

(event Custom|RangedAttack
  ;[1 1 1] TRUE = Enemy can see player
  (if (< (Transformation|GetDistanceTo (Game|Player|GetPlayerPawn 0) (Variables|Default|GetPossessed%20Pawn)) (Variables|Default|GetRangedAttackRange))
    (AI|Components|Blackboard|SetValueasBool (Variables|Default|GetBlackboard) (Variables|Default|GetShouldShoot) true)
    (else
      (AI|Components|Blackboard|SetValueasBool (Variables|Default|GetBlackboard) (Variables|Default|GetShouldShoot) false))))

(event EventPossess
  (params (PossessedPawn :type Pawn%20Object%20Reference))
  (Variables|Default|SetPossessed%20Pawn PossessedPawn)
  (AI|RunBehaviorTree "/Game/Blueprints/Enemy/Shooter/BT_ShooterEnemy.BT_ShooterEnemy"))

(fn ConstructionScript)