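; Shooter enemy Blueprint that fires projectiles at the player and cleans them up on arena activation.
; Shoot yaws the actor toward the player pawn and spawns a BP_EnemyProjectile at ShootArrow, aimed at the player with the enemy as instigator.
; Each projectile is tracked in BulletsShooted.
; Activate calls the parent logic, then destroys surviving projectiles and clears the list ahead of a level reset.
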(event EventShoot
  (bind _returnvalue (Game|Player|GetPlayerPawn 0))
  (bind _shootarrow (Variables|Default|GetShootArrow))
  (bind _returnvalue_2 (Transformation|GetWorldLocation _shootarrow))
  (bind _returnvalue_3 (Transformation|GetActorLocation _returnvalue))
  (bind _returnvalue_4 (Math|Rotator|FindLookatRotation _returnvalue_2 _returnvalue_3))
  ;[1 1 1] Shoot to player
  (Transformation|SetActorRotation (Math|Rotator|MakeRotator 0.0 0.0 (.yaw _returnvalue_4)))
  (bind _returnvalue_5 (Game|SpawnActorfromClass "/Game/Blueprints/Enemy/Shooter/BP_EnemyProjectile.BP_EnemyProjectile_C" (Math|Transform|MakeTransform _returnvalue_2 (Math|Rotator|MakeRotator (.roll _returnvalue_4) (.pitch _returnvalue_4) (.yaw _returnvalue_4)) "1,1,1") "AlwaysSpawn" 0 self))
  (Utilities|Array|Add (Variables|Default|GetBulletsShooted) _returnvalue_5))

(event EventActivate
  (params (ActualArenaIndex :type Integer))
  (bind _bulletsshooted (Variables|Default|GetBulletsShooted))
  ;[1 1 1] Destroy all projectile the enemy has shooted before reset level
  (|CallParentFunction ActualArenaIndex)
  (for _array_element _bulletsshooted
    (Utilities|IsValid _array_element
      (:Is%20Valid
        (Actor|DestroyActor _array_element))))
  (Utilities|Array|Clear _bulletsshooted))

(fn ConstructionScript
  (|CallParentFunction))