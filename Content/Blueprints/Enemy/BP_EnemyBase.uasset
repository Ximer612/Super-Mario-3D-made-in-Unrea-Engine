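; Base enemy character that patrols a list of pathfinding targets, damages the player on capsule contact and can die.
; It starts at a random target and cycles through the list, writing each location to the Blackboard.
; At zero health it is hidden and disabled rather than destroyed, notifies the player and may spawn a random pickup.
; Activate resets it to its start transform for qualifying arena indices and removes that pickup.
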(event OnComponentHit(CapsuleComponent)
  (params (HitComponent :type Primitive%20Component%20Object%20Reference) (OtherActor :type Actor%20Object%20Reference) (OtherComp :type Primitive%20Component%20Object%20Reference) (NormalImpulse :type Vector :default "0, 0, 0") (Hit :type Hit%20Result%20Structure%20%28by%20ref%29))
  ;[1 1 1] Damage player
  (if (Actor|ActorHasTag OtherActor "Player")
    (Game|Damage|ApplyDamage OtherActor 1.0 0 0)))

(event Custom|SpawnRandomPickupOrNone
  (params (NewPickupTransform :type Transform))
  (bind _pickupitemsactors (Variables|Default|GetPickupItemsActors))
  ;[1 1 1] Summon random pickup
  (if (> (Math|Random|RandomInteger 100) 60)
    (bind _returnvalue (Game|SpawnActorfromClass (Utilities|Array|Get(acopy) _pickupitemsactors (Math|Random|RandomInteger (Utilities|Array|Length _pickupitemsactors))) NewPickupTransform "AlwaysSpawn" 0 0))
    (Variables|Default|SetSpawnedPickupItem _returnvalue)))

(event Custom|Death
  ;[1 1 1] When an enemy dies
  (Class|IKillable|KilledEnemy(Message) (Game|Player|GetPlayerPawn 0))
  (CallFunction|SpawnRandomPickuporNone (Transformation|GetWorldTransform (Variables|Collision|GetCapsuleComponent))))

(event Custom|GetConsecutiveTarget
  ;[1 1 1] Get consecutive target to go with path find
  (CallFunction|SetTargetPosition)
  (bind _result (Math|Integer|IncrementInt (Variables|Custom|GetTarget%20Index))
    (:%20%20
      (Variables|Custom|SetTarget%20Index (Math|Integer|%(Integer) _result (Utilities|Array|Length (Variables|Custom|GetPathfindingTargets)))))))

(event Game|Damage|EventAnyDamage
  (params (Damage :type Float%20%28single-precision%29) (DamageType :type Damage%20Type%20Object%20Reference) (InstigatedBy :type Controller%20Object%20Reference) (DamageCauser :type Actor%20Object%20Reference))
  ;[1 1 1] Take Damage
  (bind _output_get (Variables|Default|SetHealth (- (Variables|Default|GetHealth) Damage)))
  (if (<= _output_get 0.0)
    (CallFunction|Deactivate)
    (CallFunction|Death)))

(event EventBeginPlay
  ;[1 1 1] BEGIN PLAY = get start transform, blackboard, random target, set health
  (Variables|Custom|SetStartTransform (Transformation|GetActorTransform))
  (Variables|Default|SetMyBlackboard (AI|GetBlackboard (Pawn|GetController)))
  (Variables|Custom|SetTarget%20Index (Math|Random|RandomInteger (Utilities|Array|Length (Variables|Custom|GetPathfindingTargets))))
  (Variables|Default|SetHealth (Variables|Default|GetMaxHealth)))

(event EventActivate
  (params (ActualArenaIndex :type Integer))
  (bind _spawnedpickupitem (Variables|Default|GetSpawnedPickupItem))
  ;[1 1 1] Enable / Disable
  (if (<= ActualArenaIndex (Variables|Custom|GetMyArenaIndex))
    (Transformation|SetActorTransform (Variables|Custom|GetStartTransform))
    (Development|SetHiddeninGame (Variables|Character|GetMesh) false false)
    (Collision|SetCollisionEnabled (Variables|Collision|GetCapsuleComponent) "QueryAndPhysics")
    (Pawn|Components|CharacterMovement|SetMovementMode (Variables|Character|GetCharacterMovement) "MOVE_Walking" 0)
    (AI|Components|Blackboard|SetValueasBool (AI|GetBlackboard self) (Variables|Default|GetDeactivated?) false)
    (Variables|Default|SetHealth (Variables|Default|GetMaxHealth))
    (Utilities|IsValid _spawnedpickupitem
      (:Is%20Valid
        (Actor|DestroyActor _spawnedpickupitem)))))

(event EventDeactivate
  ;[1 1 1] Enable / Disable
  (Development|SetHiddeninGame (Variables|Character|GetMesh) true false)
  (Collision|SetCollisionEnabled (Variables|Collision|GetCapsuleComponent) "NoCollision")
  (Pawn|Components|CharacterMovement|DisableMovement (Variables|Character|GetCharacterMovement))
  (AI|Components|Blackboard|SetValueasBool (AI|GetBlackboard self) (Variables|Default|GetDeactivated?) true))

(fn ConstructionScript)

(fn SetTargetPosition
  (if (> (Utilities|Array|Length (Variables|Custom|GetPathfindingTargets)) 0)
    (AI|Components|Blackboard|SetValueasVector (Variables|Default|GetMyBlackboard) (Variables|Custom|GetTargetLocation) (Transformation|GetActorLocation (Utilities|Array|Get(acopy) (Variables|Custom|GetPathfindingTargets) (Variables|Custom|GetTarget%20Index))))))