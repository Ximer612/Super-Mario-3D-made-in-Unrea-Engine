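; BP_ArenasController manages arena progression, opening a sequence of doors as coin and enemy counts reach each door's requirements.
; CheckForNextArena compares current counts to the active door's thresholds, then opens it, zeroes counts, advances indices and signals a new area or all arenas ended.
; Actors implementing I_Deactivable are cached at BeginPlay, and ResetAll reactivates them with the current arena index, clearing counts and reloading door requirements.
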(event Custom|CheckForNextArena
  ;[1 1 1] CheckVariables
  (if (not (Variables|Default|GetAreAllArenasCompleted?))
    (if (>= (Variables|Default|GetActualCoins) (Variables|Default|GetCoinsToNextArena))
      (if (>= (Variables|Default|GetActualEnemies) (Variables|Default|GetEnemiesToNextArena))
        ;[1 1 1] New Arena Unlocked
        (Variables|Default|SetActualCoins 0)
        (Variables|Default|SetActualEnemies 0)
        (Math|Integer|IncrementInt (Variables|Default|GetActualArenaIndex)
          (:%20%20
            (Default|Open (Utilities|Array|Get(acopy) (Variables|Default|GetDoorsToOpen) (Variables|Default|GetActualDoorIndex)))
            (Math|Integer|IncrementInt (Variables|Default|GetActualDoorIndex)
              (:%20%20
                (Utilities|IsValid (Utilities|Array|Get(acopy) (Variables|Default|GetDoorsToOpen) (Variables|Default|GetActualDoorIndex))
                  (:Is%20Valid
                    (CallFunction|GetDoorVariables)
                    (Default|CallNewAreaUnlocked))
                  (:Is%20Not%20Valid
                    (Variables|Default|SetAreAllArenasCompleted? true)
                    (Default|CallAllArenasEnded)))))))))))

(event Custom|GetDoorVariables
  (bind _actualdoorindex (Variables|Default|GetActualDoorIndex))
  (bind _doorstoopen (Variables|Default|GetDoorsToOpen))
  (bind _output (Utilities|Array|Get(acopy) _doorstoopen _actualdoorindex))
  ;[1 1 1] Get Door Variables to check
  (Variables|Default|SetCoinsToNextArena (Variables|/Game/Blueprints/WorldBuilding/BP_DoubleDoor.BP_DoubleDoor_C|GetCoinsToOpen _output))
  (Variables|Default|SetEnemiesToNextArena (Variables|/Game/Blueprints/WorldBuilding/BP_DoubleDoor.BP_DoubleDoor_C|GetEnemiesToOpen _output)))

(event Custom|ResetAll
  ;[1 1 1] Re-activate all actors that has been deactivated
  (for _array_element (Variables|Default|GetDeactivableActors)
    (Class|IDeactivable|Activate(Message) _array_element (Variables|Default|GetActualArenaIndex))
    (Variables|Default|SetActualCoins 0)
    (Variables|Default|SetActualEnemies 0)
    (if (not (Variables|Default|GetAreAllArenasCompleted?))
      (CallFunction|GetDoorVariables))))

(event EventBeginPlay
  ;[1 1 1] BEGIN PLAY - Get first door and get all actors that can be deactivated
  (CallFunction|GetDoorVariables)
  (bind _outactors (Actor|GetAllActorswithInterface "/Game/Blueprints/I_Deactivable.I_Deactivable_C"))
  (Variables|Default|SetDeactivableActors _outactors))

(fn ConstructionScript)